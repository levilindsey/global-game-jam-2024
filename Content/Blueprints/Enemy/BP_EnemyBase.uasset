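; Base top-down sprite enemy that initializes speed, patrol and chase tuning per type from GS_TopDown configs.
; Tick updates throttled four-diagonal facing, writes player proximity to the Blackboard and timestamps last sight and closeness.
; Fart overlaps apply a timed "disgust" slow, replaced only by stronger ones, with sound, tint and walk-speed recalculation from stacked multipliers.
; Launched and Landed toggle the airborne state and capsule physics simulation.
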(event `SetUpDebug`
  ;[1 0.8668 0.1406] DEBUG STUFF
)

(event `self.ReceiveTick`
  (params (DeltaSeconds :type "Float (single-precision)"))
  (bind _returnvalue (`AIBlueprintHelperLibrary.GetBlackboard` null))
  (bind _returnvalue_2 (`GameplayStatics.GetTimeSeconds`))
  (`SceneComponent.K2_SetRelativeLocation` (`self.Sprite`) (0.0 7.0 0.0) false false)
  (`self.K2_SetActorRotation` (struct))
  (`self.UpdateDisgust`)
  (`self.UpdateDirectionality`)
  (`self.UpdateIsCloseToPlayer`)
  (`|ExecutionSequence`
    (:`then_0`
      (if (`BlackboardComponent.GetValueAsBool` _returnvalue (`self.HasLineOfSight`))
        (set `self.LastTimeWithHasLineOfSight` _returnvalue_2)))
    (:`then_1`
      (if (`BlackboardComponent.GetValueAsBool` _returnvalue (`self.IsCloseToPlayerKey`))
        (set `self.LastTimeWithIsCloseToPlayer` _returnvalue_2)))))

(event `self.ReceiveBeginPlay`
  (`self.SetUpDebug`))

(event `OnFartOverlapStarted`
  (params (SlowDownMultplier :type "Float (double-precision)") (SlowDownDuration :type "Float (double-precision)"))
  (if (`self.IsDisgusted`)
    (if (> (`self.SlowDownMultiplier`) SlowDownMultplier)
      (set `self.SlowDownMultiplier` SlowDownMultplier :!label _label)
      (set `self.SlowDownEndTime` (+ (`GameplayStatics.GetTimeSeconds`) SlowDownDuration))
      (set `self.IsDisgusted` true)
      (`self.OnDisgustedStarted`))
    (else
      (goto _label))))

(event `OnDisgustedStarted`
  (`self.UpdateSpeed`)
  (`GameplayStatics.PlaySound2D` "/Game/Sounds/Disgusted/Disgusted_Cue.Disgusted_Cue" 1.0 1.0 0.0 null null)
  (`PaperFlipbookComponent.SetSpriteColor` (`self.Sprite`) (`self.DisgustedColor`)))

(event `OnDisgustedFinished`
  (set `self.SlowDownMultiplier` 1.0)
  (set `self.SlowDownEndTime` -100.0)
  (`self.UpdateSpeed`)
  (`PaperFlipbookComponent.SetSpriteColor` (`self.Sprite`) (`self.NormalColor`)))

(event `Launched`
  (set `self.IsAirborne` true)
  (`PrimitiveComponent.SetSimulatePhysics` (`self.CapsuleComponent`) true))

(event `Landed`
  (bind _capsulecomponent (`self.CapsuleComponent`))
  (set `self.IsAirborne` false)
  (`PrimitiveComponent.SetSimulatePhysics` _capsulecomponent false)
  (`PrimitiveComponent.SetEnableGravity` _capsulecomponent true))

(fn `SetUp`
  (params (Type :type "/Game/Blueprints/Enemy/E_EnemyType Enum" :default "NewEnumerator0"))
  (bind _asgs_top_down (cast `/Game/Blueprints/GS_TopDown` (`GameplayStatics.GetGameState`)))
  (bind _value (`BlueprintMapLibrary.Map_Find` (`/Game/Blueprints/GS_TopDown.EnemyConfigs` _asgs_top_down) Type))
  (set `self.BaseSpeed` (break `/Game/Blueprints/Enemy/S_EnemyConfig` _value))
  (set `self.BasePauseDelay` (`self.PauseDelay`))
  (set `self.ChasingChaseSpeedMultiplier` (`.ChaseSpeedMultiplier_18_BDB05DA741176F27133BB7BC939575BC` (break `/Game/Blueprints/Enemy/S_EnemyConfig` _value)))
  (set `self.PatrolRadius` (`.TODOPatrolRadius_16_9323DB0D4E2F002D22D099A4E33225FD` (break `/Game/Blueprints/Enemy/S_EnemyConfig` _value)))
  (set `self.GiveUpDelayMultiplier` (`.GiveUpDelayMultiplier_8_8BC4DFEA409E5437F964D7B086D3CFDF` (break `/Game/Blueprints/Enemy/S_EnemyConfig` _value)))
  (set `self.BaseIsCloseToPlayerThreshold` (`.IsCloseToPlayerThreshold_13_5D8C417E4D497D20C0E8888AB984E59B` (break `/Game/Blueprints/Enemy/S_EnemyConfig` _value)))
  (`self.UpdateSpeed`))

(fn `UpdateDirectionality`
  (locals (CurrentDirectionality :type "Vector2D Structure"))
  (bind _currentdirectionality_x (`KismetMathLibrary.BreakVector2D` (`local.CurrentDirectionality`)))
  (bind (_directionality_x _directionality_y) (`KismetMathLibrary.BreakVector2D` (`self.Directionality`)))
  (bind _velocity (`MovementComponent.Velocity` (`self.GetMovementComponent`)))
  (bind (_returnvalue_x _returnvalue_y) (`KismetMathLibrary.BreakVector2D` (`KismetMathLibrary.Normal2D` (`KismetMathLibrary.Conv_VectorToVector2D` _velocity))))
  (set `self.IsMoving` (not (`KismetMathLibrary.Vector_IsNearlyZero` _velocity)))
  (if (>= _returnvalue_x 0.0)
    (set `local.CurrentDirectionality` (`KismetMathLibrary.MakeVector2D` 1.0 _directionality_y))
    (else
      (set `local.CurrentDirectionality` (`KismetMathLibrary.MakeVector2D` -1.0 _directionality_y))))
  (if (>= _returnvalue_y 0.0)
    (set `local.CurrentDirectionality` (`KismetMathLibrary.MakeVector2D` _currentdirectionality_x -1.0))
    (else
      (set `local.CurrentDirectionality` (`KismetMathLibrary.MakeVector2D` _currentdirectionality_x 1.0))))
  (if (and (!= (`self.Directionality`) (`local.CurrentDirectionality`)) (>= (`GameplayStatics.GetTimeSeconds`) (+ (`self.LastDirectionalityChangeTime`) (`self.DirectionalityChangeThrottlePeriod`))))
    (set `self.Directionality` (`local.CurrentDirectionality`))
    (set `self.LastDirectionalityChangeTime` (`GameplayStatics.GetTimeSeconds`))))

(fn `UpdateDisgust`
  (bind _output_get (set `self.WasDisgusted` (`self.IsDisgusted`)))
  (bind _output_get_2 (set `self.IsDisgusted` (<= (`GameplayStatics.GetTimeSeconds`) (`self.SlowDownEndTime`))))
  (if (!= _output_get_2 _output_get)
    (if (not (`self.IsDisgusted`))
      (`self.OnDisgustedFinished`))))

(fn `UpdateIsCloseToPlayer`
  (locals (IsCloseToPlayer :type Name :default "IsCloseToPlayer"))
  (bind _asgs_top_down (cast `/Game/Blueprints/GS_TopDown` (`GameplayStatics.GetGameState`)))
  (`BlackboardComponent.SetValueAsBool` (`AIBlueprintHelperLibrary.GetBlackboard` null) (`local.IsCloseToPlayer`) (<= (`KismetMathLibrary.Vector_DistanceSquared` (`self.K2_GetActorLocation`) (`self.K2_GetActorLocation` (`GameplayStatics.GetPlayerCharacter` 0))) (`KismetMathLibrary.Square` (* (`self.BaseIsCloseToPlayerThreshold`) (`/Game/Blueprints/GS_TopDown.GlobalEnemyIsCloseToPlayerThresholdMultiplier` _asgs_top_down))))))

(fn `UpdateSpeed`
  (bind _asgs_top_down (cast `/Game/Blueprints/GS_TopDown` (`GameplayStatics.GetGameState`)))
  (set `CharacterMovementComponent.MaxWalkSpeed` (* (`self.BaseSpeed`) (`self.SlowDownMultiplier`) (`self.SpeedMultiplier`) (`self.BalanceSpeedMultiplier`) (`/Game/Blueprints/GS_TopDown.GlobalEnemySpeedMultiplier` _asgs_top_down)) (`self.CharacterMovement`)))

(fn `UserConstructionScript`)