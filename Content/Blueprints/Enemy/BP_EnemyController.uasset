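; AI controller for enemies that runs BT_Enemy on possession and feeds its Blackboard.
; BeginPlay stores the player and the controlled enemy as keys.
; Tick copies the enemy's disgusted and airborne flags and the player's last ground position into the Blackboard.
; Perception sets HasLineOfSight when the player is sensed, otherwise starts a LineOfSightTimer delay before clearing it, giving a grace period after sight is lost.
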(event `self.ReceiveBeginPlay`
  (`BlackboardComponent.SetValueAsObject` (`self.Blackboard`) (`self.PlayerActor`) (`GameplayStatics.GetPlayerCharacter` 0))
  (`BlackboardComponent.SetValueAsObject` (`self.Blackboard`) (`self.EnemyActor`) (`BlackboardComponent.GetValueAsObject` (`self.Blackboard`) (`self.SelfActor`))))

(event `self.ReceivePossess`
  (params (PossessedPawn :type "Pawn Object Reference"))
  (`self.RunBehaviorTree` "/Game/Blueprints/Enemy/BT_Enemy.BT_Enemy"))

(event `self.ReceiveTick`
  (params (DeltaSeconds :type "Float (single-precision)"))
  (bind _asbp_enemy_base (cast `/Game/Blueprints/Enemy/BP_EnemyBase` (`BlackboardComponent.GetValueAsObject` (`self.Blackboard`) (`self.SelfActor`))))
  (`BlackboardComponent.SetValueAsBool` (`self.Blackboard`) (`self.IsDisgusted`) (`/Game/Blueprints/Enemy/BP_EnemyBase.IsDisgusted` _asbp_enemy_base))
  (`BlackboardComponent.SetValueAsBool` (`self.Blackboard`) (`self.IsAirborne`) (`/Game/Blueprints/Enemy/BP_EnemyBase.IsAirborne` _asbp_enemy_base))
  (bind _asbp_player (cast `/Game/Blueprints/Player/BP_Player` (`GameplayStatics.GetPlayerCharacter` 0)))
  (`BlackboardComponent.SetValueAsVector` (`self.Blackboard`) (`self.PlayerLastGroundPosition`) (`/Game/Blueprints/Player/BP_Player.LastGroundPosition` _asbp_player)))

(event `self.AIPerception.OnTargetPerceptionUpdated`
  (params (Actor :type "Actor Object Reference") (Stimulus :type "AIStimulus Structure"))
  (if (and (`self.ActorHasTag` Actor "Player") (`.bSuccessfullySensed` (break `AIStimulus` Stimulus)))
    (`KismetSystemLibrary.K2_ClearAndInvalidateTimerHandle` (`self.EnemyTimer`))
    (`BlackboardComponent.SetValueAsBool` (`self.Blackboard`) (`self.HasLineOfSight`) true)
    (else
      (bind _returnvalue (`KismetSystemLibrary.K2_SetTimerDelegate` (delegate `PerceptionLostTimedOut`) (`self.LineOfSightTimer`)))
      (set `self.EnemyTimer` _returnvalue))))

(event `PerceptionLostTimedOut`
  (`BlackboardComponent.SetValueAsBool` (`self.Blackboard`) (`self.HasLineOfSight`) false))

(fn `UserConstructionScript`)