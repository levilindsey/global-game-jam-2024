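; BP_DashFart is a fart ability Blueprint that makes the player perform a fart-powered dash.
; On start it runs the parent logic, then calls FartDash on the Player, passing strength, duration, airborne speed multiplier and jump height ratio.
; A timer set by function name calls OnFinished after the same duration, which defers to the parent's finish logic.
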(event `self.OnStarted`
  (bind _duration (`self.Duration`))
  (`parent.OnStarted`)
  (`/Game/Blueprints/Player/BP_Player.FartDash` (`self.Player`) (`self.Strength`) _duration (`self.AirborneSpeedMultiplier`) (`self.JumpHeightRatio`))
  (`KismetSystemLibrary.K2_SetTimer` null "OnFinished" _duration))

(event `self.OnFinished`
  (`parent.OnFinished`))

(fn `UserConstructionScript`
  (`parent.UserConstructionScript`))