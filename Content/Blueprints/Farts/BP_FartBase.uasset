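; Base fart cloud actor that slows the player, slows and knocks back enemies, then destroys itself after a configured duration.
; SetUp applies the config to the flipbook and replays overlaps cached before setup; Start plays particles and sound and sets end times.
; Tick lerps the overlap sphere's radius, toggles timed effect states and pins the actor at its spawn location.
; Each enemy is affected once, with grounded ones launched by impulse.
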(event `self.ReceiveTick`
  (params (DeltaSeconds :type "Float (single-precision)"))
  (bind _startlocation (`self.StartLocation`))
  (`self.UpdateProgress`)
  (`self.UpdateRadius`)
  (`self.UpdateEnemyPushes`)
  (`self.UpdatePlayerSlowDown`)
  (if (!= (`self.K2_GetActorLocation`) _startlocation)
    (`self.K2_SetActorLocation` _startlocation false true)))

(event `self.ReceiveBeginPlay`
  (set `self.StartLocation` (`self.K2_GetActorLocation`)))

(event `self.ReceiveActorBeginOverlap`
  (params (OtherActor :type "Actor Object Reference"))
  (bind _asbp_enemy_base (cast `/Game/Blueprints/Enemy/BP_EnemyBase` OtherActor))
  (if (not (`BlueprintSetLibrary.Set_Contains` (`self.CollidedEnemies`) _asbp_enemy_base))
    (`BlueprintSetLibrary.Set_Add` (`self.CollidedEnemies`) _asbp_enemy_base)
    (bind _issetup (`self.GetIsSetUp`))
    (if _issetup
      (`self.HandleEnemyOverlap` _asbp_enemy_base))))

(event `OnStarted`
  (bind (_config_type _config_duration) (break `/Game/Blueprints/Farts/S_FartConfig` (`self.Config`)))
  (`KismetSystemLibrary.Delay` _config_duration)
  (`self.OnFinished`))

(event `OnFinished`
  (`self.OnFinishedSlowingPlayer`)
  (`self.K2_DestroyActor`))

(event `OnStartedSlowingPlayer`
  (bind (_config_type _config_duration _config_cooldown _config_flipbook _config_icon _config_sounds _config_class _config_enemypushbackstrength _config_enemypushbackduration _config_playerslowdownmultiplier) (break `/Game/Blueprints/Farts/S_FartConfig` (`self.Config`)))
  (set `/Game/Blueprints/Player/BP_Player.SpeedMultiplier` (`KismetMathLibrary.FMin` (`/Game/Blueprints/Player/BP_Player.SpeedMultiplier` (`self.Player`)) _config_playerslowdownmultiplier) (`self.Player`)))

(event `OnFinishedSlowingPlayer`
  (bind (_config_type _config_duration _config_cooldown _config_flipbook _config_icon _config_sounds _config_class _config_enemypushbackstrength _config_enemypushbackduration _config_playerslowdownmultiplier) (break `/Game/Blueprints/Farts/S_FartConfig` (`self.Config`)))
  (if (== (`/Game/Blueprints/Player/BP_Player.SpeedMultiplier` (`self.Player`)) _config_playerslowdownmultiplier)
    (set `/Game/Blueprints/Player/BP_Player.SpeedMultiplier` 1.0 (`self.Player`))))

(event `OnStartedPushingEnemies`)

(event `OnFinishedPushingEnemies`)

(fn `GetIsSetUp`
  (returns (IsSetUp :type Boolean))
  (bind (_config_type _config_duration) (break `/Game/Blueprints/Farts/S_FartConfig` (`self.Config`)))
  (return (!= _config_duration 0.0)))

(fn `HandleEnemyOverlap`
  (params (Enemy :type "/Game/Blueprints/Enemy/BP_EnemyBase Object Reference"))
  (bind _returnvalue (`self.K2_GetActorLocation` Enemy))
  (bind _capsulecomponent (`Character.CapsuleComponent` Enemy))
  (bind (_config_type _config_duration _config_cooldown _config_flipbook _config_icon _config_sounds _config_class _config_enemypushbackstrength _config_enemypushbackduration _config_playerslowdownmultiplier _config_playerslowdownduration _config_enemyslowdownmultiplier _config_enemyslowdownduration) (break `/Game/Blueprints/Farts/S_FartConfig` (`self.Config`)))
  (`KismetSystemLibrary.PrintString` "Fart touched enemy." false true (struct :`R` 0.846084 :`B` 1.0 :`A` 1.0))
  (`/Game/Blueprints/Enemy/BP_EnemyBase.OnFartOverlapStarted` Enemy _config_enemyslowdownmultiplier _config_enemyslowdownduration)
  (if (not (`/Game/Blueprints/Enemy/BP_EnemyBase.IsAirborne` Enemy))
    (`/Game/Blueprints/Enemy/BP_EnemyBase.Launched` Enemy)
    (`PrimitiveComponent.AddVelocityChangeImpulseAtLocation` _capsulecomponent (* (`.EnemyPushBackStrength_56_475EC2F8465CCDEA0D0761850C9E8DDC` (break `/Game/Blueprints/Farts/S_FartConfig` (`self.Config`))) (`KismetMathLibrary.MakeVector` (.x (`KismetMathLibrary.Normal` (- _returnvalue (`self.K2_GetActorLocation`)))) (.y (`KismetMathLibrary.Normal` (- _returnvalue (`self.K2_GetActorLocation`)))) 0.05)) _returnvalue "None")
    (`PrimitiveComponent.SetEnableGravity` _capsulecomponent false)
    (`self.K2_SetActorLocation` (+ _returnvalue (`KismetMathLibrary.MakeVector` 0.0 0.0 4.0)) false true)
    (`KismetSystemLibrary.K2_SetTimer` Enemy "Landed" 0.2)))

(fn `SetUp`
  (params (Config :type "/Game/Blueprints/Farts/S_FartConfig Structure") (Player :type "/Game/Blueprints/Player/BP_Player Object Reference"))
  (bind _paperflipbook (`self.PaperFlipbook`))
  (set `self.Player` Player)
  (bind _output_get (set `self.Config` Config))
  (bind (_type _duration _cooldown _flipbook _icon _sounds _class _enemypushbackstrength _enemypushbackduration _playerslowdownmultiplier _playerslowdownduration _enemyslowdownmultiplier _enemyslowdownduration _startradius _endradius _cantriggerinair _usescount _particleplaybackrate _particlescale) (break `/Game/Blueprints/Farts/S_FartConfig` _output_get))
  (`SceneComponent.SetRelativeScale3D` _paperflipbook (* (* _particlescale (`self.BaseScale`)) (`KismetMathLibrary.Vector_One`)))
  (`PaperFlipbookComponent.SetPlayRate` _paperflipbook _particleplaybackrate)
  (`PaperFlipbookComponent.SetFlipbook` _paperflipbook _flipbook)
  (bind _result (`BlueprintSetLibrary.Set_ToArray` (`self.CollidedEnemies`)))
  (for _array_element _result
    (`self.HandleEnemyOverlap` _array_element)))

(fn `Start`
  (params (Config :type "/Game/Blueprints/Farts/S_FartConfig Structure"))
  (bind (_type _duration _cooldown _flipbook _icon _sounds _class _enemypushbackstrength _enemypushbackduration _playerslowdownmultiplier _playerslowdownduration) (break `/Game/Blueprints/Farts/S_FartConfig` Config))
  (bind _returnvalue (`GameplayStatics.GetTimeSeconds`))
  (bind _asgs_top_down (cast `/Game/Blueprints/GS_TopDown` (`GameplayStatics.GetGameState`)))
  (`/Game/Blueprints/GS_TopDown.PlayOneShotParticles` _asgs_top_down (`self.PaperFlipbook`))
  (`GameplayStatics.PlaySoundAtLocation` _sounds (`self.K2_GetActorLocation`) (struct) 1.0 1.0 0.0 null null null null)
  (set `self.EndTime` (+ _duration _returnvalue))
  (set `self.StartTime` _returnvalue)
  (set `self.EnemyPushBackEndTime` (+ _returnvalue _enemypushbackduration))
  (set `self.PlayerSlowDownEndTime` (+ _returnvalue _playerslowdownduration))
  (`self.OnStarted`))

(fn `UpdateEnemyPushes`
  (bind _output_get (set `self.WasPushingEnemies` (`self.IsPushingEnemies`)))
  (bind _output_get_2 (set `self.IsPushingEnemies` (>= (`self.EnemyPushBackEndTime`) (`GameplayStatics.GetTimeSeconds`))))
  (if (!= _output_get_2 _output_get)
    (if (`self.IsPushingEnemies`)
      (`self.OnStartedPushingEnemies`)
      (else
        (`self.OnFinishedPushingEnemies`)))))

(fn `UpdatePlayerSlowDown`
  (bind _output_get (set `self.WasSlowingPlayer` (`self.IsSlowingPlayer`)))
  (bind _output_get_2 (set `self.IsSlowingPlayer` (>= (`self.PlayerSlowDownEndTime`) (`GameplayStatics.GetTimeSeconds`))))
  (if (!= _output_get_2 _output_get)
    (if (`self.IsSlowingPlayer`)
      (`self.OnStartedSlowingPlayer`)
      (else
        (`self.OnFinishedSlowingPlayer`)))))

(fn `UpdateProgress`
  (set `self.Progress` (/ (- (`GameplayStatics.GetTimeSeconds`) (`self.StartTime`)) (- (`self.EndTime`) (`self.StartTime`)))))

(fn `UpdateRadius`
  (bind (_config_type _config_duration _config_cooldown _config_flipbook _config_icon _config_sounds _config_class _config_enemypushbackstrength _config_enemypushbackduration _config_playerslowdownmultiplier _config_playerslowdownduration _config_enemyslowdownmultiplier _config_enemyslowdownduration _config_startradius _config_endradius) (break `/Game/Blueprints/Farts/S_FartConfig` (`self.Config`)))
  (`SphereComponent.SetSphereRadius` (`self.OverlapRegion`) (`KismetMathLibrary.Lerp` _config_startradius _config_endradius (`self.Progress`)) true))

(fn `UserConstructionScript`)