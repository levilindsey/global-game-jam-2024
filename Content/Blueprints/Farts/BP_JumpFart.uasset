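; BP_JumpFart is a fart ability that launches the player into a fart-powered jump.
; On start it calls the player's FartJump with its strength, airborne speed multiplier and jump height ratio, plus a duration looked up in the GS_TopDown game state's FartConfigs map.
; It then sets a timer by function name for OnFinished, which only runs the parent's finish logic.
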(event `self.OnStarted`
  (`parent.OnStarted`)
  (bind _asgs_top_down (cast `/Game/Blueprints/GS_TopDown` (`GameplayStatics.GetGameState`)))
  (`/Game/Blueprints/Player/BP_Player.FartJump` (`self.Player`) (`self.Strength`) (`.Duration_8_EF778B2E449704EEA68C39BF69F0ECF8` (break `/Game/Blueprints/Farts/S_FartConfig` (`BlueprintMapLibrary.Map_Find` (`/Game/Blueprints/GS_TopDown.FartConfigs` _asgs_top_down) "NewEnumerator1"))) (`self.AirborneSpeedMultiplier`) (`self.JumpHeightRatio`))
  (`KismetSystemLibrary.K2_SetTimer` null "OnFinished" 0.0))

(event `self.OnFinished`
  (`parent.OnFinished`))

(fn `UserConstructionScript`
  (`parent.UserConstructionScript`))