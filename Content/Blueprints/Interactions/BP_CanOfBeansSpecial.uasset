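; Special bean can pickup, built on a parent interaction class that it configures on BeginPlay with sound, particles, one-time and cooldown settings.
; When triggered while alive, it checks that the player can pick up beans and awards them before calling TryTrigger.
; If that succeeds, it hides the can, destroys itself and plays a special 2D sound.
; Tick bobs the can along relative Y using a repeating half-sine of game time.
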(event `self.ReceiveBeginPlay`
  (`parent.ReceiveBeginPlay`)
  (`self.SetUp` (`self.Sound`) (`self.Particles`) (`self.LookParticles`) (`self.IsOneTime`) (`self.Cooldown`))
  (set `self.SpriteStartPosition` (`SceneComponent.RelativeLocation` (`self.Can`))))

(event `self.Trigger`
  (params (Player :type "/Game/Blueprints/Player/BP_Player Object Reference"))
  (if (`self.IsAlive`)
    (bind _canpickup (`/Game/Blueprints/Player/BP_Player.GetCanPickUpBeans` Player))
    (if _canpickup
      (`/Game/Blueprints/Player/BP_Player.PickUpBeans` Player true)
      (bind _triggered (`self.TryTrigger` Player))
      (if _triggered
        (`SceneComponent.SetVisibility` (`self.Can`) false false)
        (`self.Destroy`)
        (`GameplayStatics.PlaySound2D` "/Game/Sounds/SpecialCan.SpecialCan" 1.0 1.0 0.0 null null)))))

(event `self.ReceiveTick`
  (params (DeltaSeconds :type "Float (single-precision)"))
  (bind _bobperiod (`self.BobPeriod`))
  (bind (_spritestartposition_x _spritestartposition_y _spritestartposition_z) (`KismetMathLibrary.BreakVector` (`self.SpriteStartPosition`)))
  (bind _boboffset (`self.BobOffset`))
  (`SceneComponent.K2_SetRelativeLocation` (`self.Can`) (`KismetMathLibrary.MakeVector` _spritestartposition_x (+ _spritestartposition_y (+ (* (* (`KismetMathLibrary.Sin` (* (/ (mod (`GameplayStatics.GetTimeSeconds`) _bobperiod) _bobperiod) (`KismetMathLibrary.GetPI`))) -1.0) (* 2.0 _boboffset)) (* _boboffset 1.0))) _spritestartposition_z) false false))

(fn `UserConstructionScript`
  (`parent.UserConstructionScript`))