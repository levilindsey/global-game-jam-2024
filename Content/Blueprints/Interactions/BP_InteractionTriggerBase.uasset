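; Base actor for player-triggered interactions, configured by child or caller through SetUp.
; TryTrigger enforces one-time and cooldown rules, plays a sound, and fires one-shot particles through GS_TopDown, marking the actor dead when those particles are valid.
; Look-at changes toggle looping highlight particles via the game state, only while the player can pick up beans.
; Destroy hides the highlight, then removes the actor after a short timer.
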(event `Trigger`
  (params (Player :type "/Game/Blueprints/Player/BP_Player Object Reference"))
  (`self.TryTrigger` Player))

(fn `Destroy`
  (`SceneComponent.SetVisibility` (`self.BaseLookParticles`) false false)
  (`KismetSystemLibrary.K2_SetTimer` null "DestroyDelayFinished" 1.0))

(fn `DestroyDelayFinished`
  (`self.K2_DestroyActor`))

(fn `GetGameState`
  (returns (GameState :type "/Game/Blueprints/GS_TopDown Object Reference"))
  (bind _asgs_top_down (cast `/Game/Blueprints/GS_TopDown` (`GameplayStatics.GetGameState`)))
  (return _asgs_top_down))

(fn `GetHasTriggered`
  (returns (HasTriggered :type Boolean))
  (return (> (`self.BaseLastTriggerTime`) 0.0)))

(fn `SetIsLookedAt`
  (params (IsLookedAt :type Boolean))
  (locals (WasLookedAt :type Boolean))
  (bind _baselookparticles (`self.BaseLookParticles`))
  (if (`self.IsAlive`)
    (bind _asbp_player (cast `/Game/Blueprints/Player/BP_Player` (`GameplayStatics.GetPlayerCharacter` 0)))
    (bind _canpickup (`/Game/Blueprints/Player/BP_Player.GetCanPickUpBeans` _asbp_player))
    (if _canpickup
      (bind _output_get (set `local.WasLookedAt` (`self.IsLookedAt`)))
      (bind _output_get_2 (set `self.IsLookedAt` IsLookedAt))
      (if (!= _output_get_2 _output_get)
        (bind _gamestate (`self.GetGameState`))
        (`/Engine/EditorBlueprintResources/StandardMacros.IsValid` _baselookparticles
          (:`Is Valid`
            (`/Game/Blueprints/GS_TopDown.SetLoopingParticlesIsPlaying` _gamestate _baselookparticles _output_get_2))
          (:`Is Not Valid`
            _)))
      (`KismetSystemLibrary.PrintString` (`KismetStringLibrary.Concat_StrStr` (`KismetMathLibrary.SelectString` "STARTED" "STOPPED" _output_get_2) " looking at trigger.") false true (struct :`R` 0.846084 :`B` 1.0 :`A` 1.0)))))

(fn `SetUp`
  (params (Sound :type "SoundCue Object Reference") (Particles :type "PaperFlipbookComponent Object Reference") (LookParticles :type "PaperFlipbookComponent Object Reference") (IsOneTime :type Boolean) (Cooldown :type "Float (double-precision)"))
  (set `self.BaseSound` Sound)
  (set `self.BaseParticles` Particles)
  (set `self.BaseLookParticles` LookParticles)
  (set `self.BaseIsOneTime` IsOneTime)
  (set `self.BaseCooldown` Cooldown))

(fn `TryTrigger`
  (params (Player :type "/Game/Blueprints/Player/BP_Player Object Reference"))
  (returns (Triggered :type Boolean))
  (bind _basesound (`self.BaseSound`))
  (bind _baseparticles (`self.BaseParticles`))
  (if (`self.IsAlive`)
    (bind _hastriggered (`self.GetHasTriggered`))
    (if (not (and _hastriggered (`self.BaseIsOneTime`)))
      (if (>= (`GameplayStatics.GetTimeSeconds`) (+ (`self.BaseLastTriggerTime`) (`self.BaseCooldown`)))
        (set `self.BaseLastTriggerTime` (`GameplayStatics.GetTimeSeconds`))
        (`/Engine/EditorBlueprintResources/StandardMacros.IsValid` _basesound
          (:`Is Valid`
            (`GameplayStatics.PlaySoundAtLocation` _basesound (`self.K2_GetActorLocation`) (struct) 1.0 1.0 0.0 null null null null))
          (:`Is Not Valid`
            _))
        (bind _gamestate (`self.GetGameState`))
        (`/Engine/EditorBlueprintResources/StandardMacros.IsValid` _baseparticles
          (:`Is Valid`
            (`/Game/Blueprints/GS_TopDown.PlayOneShotParticles` _gamestate _baseparticles)
            (set `self.IsAlive` false))
          (:`Is Not Valid`
            _))
        (return true)
        (else
          _)))
    (return false)))

(fn `UserConstructionScript`)