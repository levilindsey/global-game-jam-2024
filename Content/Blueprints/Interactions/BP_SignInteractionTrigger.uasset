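; A sign interaction trigger Blueprint that responds when a player triggers it, currently with only a placeholder debug message.
; On BeginPlay it passes its sound, particle, look-particle, one-time and cooldown settings to SetUp.
; Trigger calls TryTrigger with the player and prints green on-screen text when that check succeeds.
; No sign-specific behavior is implemented beyond that print.
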(event `self.ReceiveBeginPlay`
  (`parent.ReceiveBeginPlay`)
  (`self.SetUp` (`self.Sound`) (`self.Particles`) (`self.LookParticles`) (`self.IsOneTime`) (`self.Cooldown`)))

(event `Trigger`
  (params (Player :type "/Game/Blueprints/Player/BP_Player Object Reference"))
  (bind _triggered (`self.TryTrigger` Player))
  (if _triggered
    (`KismetSystemLibrary.PrintString` "Poopy butt" true true (struct :`R` 0.084768 :`G` 1.0 :`A` 1.0) 4.0)))

(fn `UserConstructionScript`
  (`parent.UserConstructionScript`))