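; BP_ItemSlotState holds the player's fart item slots, tracking each one's cooldown, remaining uses and whether it can be triggered.
; SetSlotItem fills a slot from the game state's fart config and updates its HUD widget.
; Tick counts cooldowns down, while TriggerSlot restarts the cooldown, spends a use and plays the widget's consume animation.
; After a short delay, a depleted slot empties and takes slot 2's item, if any.
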(event `self.ReceiveBeginPlay`
  (bind (_output_index _output_farttype) (break `/Game/Blueprints/Player/S_ItemSlotData` (`|GetArrayItem` (`self.Slots`) 2)))
  (bind (_output_index_2 _output_farttype_2) (break `/Game/Blueprints/Player/S_ItemSlotData` (`|GetArrayItem` (`self.Slots`))))
  (bind (_output_index_3 _output_farttype_3) (break `/Game/Blueprints/Player/S_ItemSlotData` (`|GetArrayItem` (`self.Slots`) 1)))
  (`self.SetSlotItem` _output_farttype_2)
  (`self.SetSlotItem` _output_farttype_3 1)
  (`self.SetSlotItem` _output_farttype 2))

(event `self.ReceiveTick`
  (params (DeltaSeconds :type "Float (single-precision)"))
  (for (_ _array_index) (`self.Slots`)
    (`self.UpdateSlot` _array_index DeltaSeconds)))

(event `CooldownFinished`
  (params (Index :type Integer)))

(event `UsesDepleted`
  (params (Index :type Integer))
  (`KismetSystemLibrary.Delay` 0.35)
  (`self.SetSlotItem` "NewEnumerator5" Index)
  (bind _data (`self.GetSlot` 2))
  (if (`|EnumInequality` (`.FartType_22_E145F1A04CA5945F7C4608B8F584F25D` (break `/Game/Blueprints/Player/S_ItemSlotData` _data)) "NewEnumerator5")
    (`self.SetSlotItem` (`.FartType_22_E145F1A04CA5945F7C4608B8F584F25D` (break `/Game/Blueprints/Player/S_ItemSlotData` _data)) Index)
    (`self.SetSlotItem` "NewEnumerator5" 2)))

(fn `GetGameState`
  (returns (GameState :type "/Game/Blueprints/GS_TopDown Object Reference"))
  (bind _asgs_top_down (cast `/Game/Blueprints/GS_TopDown` (`GameplayStatics.GetGameState`)))
  (return _asgs_top_down))

(fn `GetSlot`
  (params (Index :type Integer))
  (returns (Data :type "/Game/Blueprints/Player/S_ItemSlotData Structure"))
  (return (`|GetArrayItem` (`self.Slots`) Index)))

(fn `GetSlotWidget`
  (params (Index :type Integer))
  (returns (Widget :type "/Game/Blueprints/UI/WBP_ItemSlot Object Reference"))
  (bind _gamestate (`self.GetGameState`))
  (bind _slot (`/Game/Blueprints/UI/WBP_HUD.GetSlotWidget` (`|ConvertAsset` (`/Game/Blueprints/GS_TopDown.HUD` _gamestate)) Index))
  (return _slot))

(fn `SetSlotItem`
  (params (Type :type "/Game/Blueprints/Farts/E_FartType Enum" :default "NewEnumerator5") (Index :type Integer))
  (locals (SlotData :type "/Game/Blueprints/Player/S_ItemSlotData Structure"))
  (bind _asgs_top_down (cast `/Game/Blueprints/GS_TopDown` (`GameplayStatics.GetGameState`)))
  (bind _config (`/Game/Blueprints/GS_TopDown.GetFartConfig` _asgs_top_down Type))
  (bind (_type _duration _cooldown _flipbook _icon _sounds _class _enemypushbackstrength _enemypushbackduration _playerslowdownmultiplier _playerslowdownduration _enemyslowdownmultiplier _enemyslowdownduration _startradius _endradius _cantriggerinair _usescount) (break `/Game/Blueprints/Farts/S_FartConfig` _config))
  (bind _structout (setmembers `/Game/Blueprints/Player/S_ItemSlotData` :`StructRef` (`|GetArrayItem` (`self.Slots`) Index) :`Index` Index :`FartType` Type :`FartConfig` _config :`MaxCooldown` _cooldown :`CurrentCooldown` 0.0 :`LastTriggerTime` -100.0 :`MaxUses` _usescount :`RemainingUses` _usescount :`CanBeTriggered` true))
  (`KismetArrayLibrary.Array_Set` (`self.Slots`) Index (`|Copy` _structout))
  (bind _widget (`self.GetSlotWidget` Index))
  (`/Game/Blueprints/UI/WBP_ItemSlot.SetItem` _widget Type))

(fn `TriggerSlot`
  (params (Index :type Integer))
  (locals (PreviousRemainingUses :type Integer))
  (bind _output (`|GetArrayItem` (`self.Slots`) Index))
  (bind (_index _farttype _fartconfig _maxcooldown _currentcooldown _lasttriggertime _maxuses _remaininguses) (break `/Game/Blueprints/Player/S_ItemSlotData` _output))
  (set `local.PreviousRemainingUses` _remaininguses)
  (bind _structout (setmembers `/Game/Blueprints/Player/S_ItemSlotData` :`StructRef` _output :`CurrentCooldown` _maxcooldown :`LastTriggerTime` (`GameplayStatics.GetTimeSeconds`) :`RemainingUses` (- _remaininguses 1) :`CanBeTriggered` true))
  (bind _widget (`self.GetSlotWidget` Index))
  (`UserWidget.PlayAnimation` _widget (`/Game/Blueprints/UI/WBP_ItemSlot.Consume` _widget) 0.0 1 "Forward" 1.0 false)
  (if (and (> (`local.PreviousRemainingUses`) 0) (== (`.RemainingUses_17_4401B46C4276B9767151A5B9D53703B0` (break `/Game/Blueprints/Player/S_ItemSlotData` _structout)) 0))
    (`self.UsesDepleted` Index)))

(fn `UpdateSlot`
  (params (Index :type Integer) (Delta :type "Float (double-precision)"))
  (locals (PreviousCooldown :type "Float (double-precision)"))
  (bind _output (`|GetArrayItem` (`self.Slots`) Index))
  (bind (_index _farttype _fartconfig _maxcooldown _currentcooldown _lasttriggertime _maxuses _remaininguses) (break `/Game/Blueprints/Player/S_ItemSlotData` _output))
  (bind _returnvalue (`KismetMathLibrary.FMax` (- _currentcooldown Delta)))
  (set `local.PreviousCooldown` _currentcooldown)
  (bind _structout (setmembers `/Game/Blueprints/Player/S_ItemSlotData` :`StructRef` _output :`CurrentCooldown` _returnvalue :`CanBeTriggered` (and (== _returnvalue 0.0) (> _remaininguses 0))))
  (if (and (> (`local.PreviousCooldown`) 0.0) (== (`.CurrentCooldown_19_B520905549F97C08A74C11B869BAED8C` (break `/Game/Blueprints/Player/S_ItemSlotData` _structout)) 0.0))
    (`self.CooldownFinished` 0)))