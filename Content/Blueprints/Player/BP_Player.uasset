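; Player pawn for a top-down sprite game, handling movement, health, interaction and bean-powered farts.
; Attack inputs trigger item slots that spawn fart actors configured by the game state; bean pickups fill empty slots.
; Jumps and dashes are timed airborne states, faked with a sine-driven sprite offset and scaled shadow.
; Overlapping non-disgusted enemies deal damage with timed red blinking, except while airborne or in the intro; death restarts the level.
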(event `self.ReceiveActorBeginOverlap`
  (params (OtherActor :type "Actor Object Reference"))
  (bind _asbp_enemy_base (cast `/Game/Blueprints/Enemy/BP_EnemyBase` OtherActor))
  (`self.OnEnemyBeginOverlap` _asbp_enemy_base))

(event `self.ReceiveActorEndOverlap`
  (params (OtherActor :type "Actor Object Reference"))
  (bind _asbp_enemy_base (cast `/Game/Blueprints/Enemy/BP_EnemyBase` OtherActor))
  (`self.OnEnemyEndOverlap` _asbp_enemy_base))

(event `SetUpDebug`
  ;[1 0.8668 0.1406] DEBUG STUFF
)

(event `self.ReceiveBeginPlay`
  (bind _gamestate (`self.GetGameState`))
  (`/Game/Blueprints/GS_TopDown.Reset` _gamestate)
  (bind _asplayer_controller (cast `PlayerController` (`self.GetController`)))
  (message `EnhancedInputSubsystemInterface.AddMappingContext` (pcsubsystem `EnhancedInputLocalPlayerSubsystem` _asplayer_controller) "/Game/Blueprints/Player/IMC_Player.IMC_Player" 0 (struct))
  (`self.SetUpDebug`)
  (`WidgetBlueprintLibrary.SetInputMode_GameOnly` (`GameplayStatics.GetPlayerController` 0)))

(event `self.ReceiveTick`
  (params (DeltaSeconds :type "Float (single-precision)"))
  (`SceneComponent.K2_SetRelativeLocation` (`self.Sprite`) (1.2 7.0 0.0) false false)
  (`self.K2_SetActorRotation` (struct))
  (if (not (`self.IsAirborne`))
    (set `self.LastGroundPosition` (`self.K2_GetActorLocation`)))
  (if (`self.IsAirborne`)
    (`self.ApplyMovement`))
  (`self.UpdateJumpHeight`)
  (`self.UpdateLookedAtTrigger`)
  (bind _isoverlapping (`self.GetIsOverlappingEnemies`))
  (if _isoverlapping
    (bind _cantakedamage (`self.GetCanTakeDamageThisFrame`))
    (if _cantakedamage
      (`self.TakeDamage`))))

(event `EnhancedInput|/Game/Blueprints/Player/IA_Move`
  (params (ActionValue :type "Vector2D Structure") (ElapsedSeconds :type "Float (double-precision)") (TriggeredSeconds :type "Float (double-precision)") (InputAction :type "InputAction Object Reference" :default "/Game/Blueprints/Player/IA_Move.IA_Move"))
  (:`Triggered`
    (set `self.Directionality` (`KismetMathLibrary.MakeVector2D` ActionValue_X ActionValue_Y))
    (if (not (`self.IsAirborne`))
      (`self.ApplyMovement`)))
  (:`Started`
    (set `self.IsHoldingMove` true))
  (:`Completed`
    (set `self.IsHoldingMove` false)))

(event `EnhancedInput|/Game/Blueprints/Player/IA_Primary`
  (params (ActionValue :type Boolean) (ElapsedSeconds :type "Float (double-precision)") (TriggeredSeconds :type "Float (double-precision)") (InputAction :type "InputAction Object Reference" :default "/Game/Blueprints/Player/IA_Primary.IA_Primary"))
  (:`Started`
    (`self.OnAttackPressed` 0)))

(event `EnhancedInput|/Game/Blueprints/Player/IA_Secondary`
  (params (ActionValue :type Boolean) (ElapsedSeconds :type "Float (double-precision)") (TriggeredSeconds :type "Float (double-precision)") (InputAction :type "InputAction Object Reference" :default "/Game/Blueprints/Player/IA_Secondary.IA_Secondary"))
  (:`Started`
    (`self.OnAttackPressed` 1)))

(event `EnhancedInput|/Game/Blueprints/Player/IA_Interact`
  (params (ActionValue :type Boolean) (ElapsedSeconds :type "Float (double-precision)") (TriggeredSeconds :type "Float (double-precision)") (InputAction :type "InputAction Object Reference" :default "/Game/Blueprints/Player/IA_Interact.IA_Interact"))
  (:`Started`
    (`self.On Interact Pressed`)))

(event `OnEnemyBeginOverlap`
  (params (Enemy :type "/Game/Blueprints/Enemy/BP_EnemyBase Object Reference"))
  (`BlueprintSetLibrary.Set_Add` (`self.OverlappingEnemies`) Enemy)
  (bind _cantakedamage (`self.GetCanTakeDamageThisFrame`))
  (if _cantakedamage
    (`self.TakeDamage`)))

(event `OnEnemyEndOverlap`
  (params (Enemy :type "/Game/Blueprints/Enemy/BP_EnemyBase Object Reference"))
  (`BlueprintSetLibrary.Set_Remove` (`self.OverlappingEnemies`) Enemy))

(event `TakeDamage`
  (set `self.LastDamageTime` (`GameplayStatics.GetTimeSeconds`))
  (set `self.CurrentHealth` (- (`self.CurrentHealth`) (`self.DamageFromEnemy`)))
  (`KismetSystemLibrary.PrintString` (`KismetStringLibrary.Concat_StrStr` "Took damage! Health: " (`KismetStringLibrary.Conv_DoubleToString` (`self.CurrentHealth`)) " / " (`KismetStringLibrary.Conv_DoubleToString` (`self.MaxHealth`))) false true (struct :`R` 1.0 :`G` 0.455539 :`A` 1.0))
  (if (<= (`self.CurrentHealth`) 0.0)
    (`self.Killed`)
    (else
      (`GameplayStatics.PlaySoundAtLocation` "/Game/Sounds/Damage/Damage_Sound.Damage_Sound" (`self.K2_GetActorLocation`) (struct) 1.0 1.0 0.0 null null null null)
      (`self.StartDamageBlink`))))

(event `Killed`
  (bind _levelrestartdelay (`self.LevelRestartDelay`))
  (set `self.IsAlive` false)
  (`GameplayStatics.PlaySoundAtLocation` "/Game/Sounds/DeathKnell_01.DeathKnell_01" (`self.K2_GetActorLocation`) (struct) 1.0 1.0 0.0 null null null null)
  (`PaperFlipbookComponent.SetSpriteColor` (`self.Sprite`) (`self.KilledColor`))
  (`KismetSystemLibrary.PrintString` "Game over!" true true (struct :`R` 1.0 :`G` 0.455539 :`A` 1.0) _levelrestartdelay)
  (`KismetSystemLibrary.PrintString` "Restarting..." true true (struct :`G` 0.66 :`B` 1.0 :`A` 1.0) _levelrestartdelay)
  (`KismetSystemLibrary.Delay` _levelrestartdelay)
  (bind _gamestate (`self.GetGameState`))
  (`GameplayStatics.OpenLevel` (`/Game/Blueprints/GS_TopDown.MainLevel` _gamestate)))

(event `Jumped`
  (params (AirborneSpeedMultiplier :type "Float (double-precision)") (JumpVelocity :type "Vector2D Structure") (Duration :type "Float (double-precision)") (JumpHeightRatio :type "Float (double-precision)"))
  (bind _returnvalue (`GameplayStatics.GetTimeSeconds`))
  (set `self.JumpHeightRatio` JumpHeightRatio)
  (set `self.JumpTime` _returnvalue)
  (set `self.LandTime` (+ _returnvalue Duration))
  (`self.ToggleAirborne` true AirborneSpeedMultiplier JumpVelocity)
  (`KismetSystemLibrary.K2_SetTimer` null "Landed" Duration)
  (`KismetSystemLibrary.PrintString` "Jumped" false true (struct :`R` 0.846084 :`B` 1.0 :`A` 1.0)))

(event `Landed`
  (set `self.JumpHeightRatio` 1.0)
  (set `self.JumpTime` -100.0)
  (set `self.LandTime` -100.0)
  (`self.ToggleAirborne` false)
  (`KismetSystemLibrary.PrintString` "Landed" false true (struct :`R` 0.846084 :`B` 1.0 :`A` 1.0)))

(fn `ApplyMovement`
  (locals (JumpMoveControlMovement :type "Vector2D Structure"))
  (bind (_returnvalue_x _returnvalue_y) (`KismetMathLibrary.BreakVector2D` (+ (`local.JumpMoveControlMovement`) (`self.JumpVelocity`))))
  (if (`self.IsAlive`)
    (if (not (`self.HasReachedGoal`))
      (if (`self.IsHoldingMove`)
        (set `local.JumpMoveControlMovement` (* (`KismetMathLibrary.Normal2D` (`self.Directionality`)) (* (* (`self.BaseSpeed`) (`self.SpeedMultiplier`)) (`self.AirborneSpeedMultiplier`))))
        (else
          (set `local.JumpMoveControlMovement` (0.0 0.0))))
      (`self.AddMovementInput` (1.0 0.0 0.0) _returnvalue_x)
      (`self.AddMovementInput` (0.0 -1.0 0.0) _returnvalue_y))))

(fn `CalculateLookedAtTrigger`
  (returns (Trigger :type "/Game/Blueprints/Interactions/BP_InteractionTriggerBase Object Reference"))
  (for _array_element (`PrimitiveComponent.GetOverlappingActors` (`self.OverlapRegion`) "/Game/Blueprints/Interactions/BP_InteractionTriggerBase.BP_InteractionTriggerBase_C")
    (bind _asbp_interaction_trigger_base (cast `/Game/Blueprints/Interactions/BP_InteractionTriggerBase` _array_element))
    (return _asbp_interaction_trigger_base)))

(fn `EndDamageBlink`
  (set `self.IsDamageBlinkRed` false)
  (set `self.IsDamageBlinkActive` false)
  (`PaperFlipbookComponent.SetSpriteColor` (`self.Sprite`) (`self.NormalColor`)))

(fn `Fart`
  (params (Type :type "/Game/Blueprints/Farts/E_FartType Enum" :default "NewEnumerator0"))
  (bind _asgs_top_down (cast `/Game/Blueprints/GS_TopDown` (`GameplayStatics.GetGameState`)))
  (bind _config (`/Game/Blueprints/GS_TopDown.GetFartConfig` _asgs_top_down Type))
  (bind _returnvalue (`|SpawnActorFromClass` (`.Class_26_B2E7001D4EB57D39282BA2A5821E7DDE` (break `/Game/Blueprints/Farts/S_FartConfig` _config)) (`self.GetTransform`) "AlwaysSpawn" "MultiplyWithRoot" null null))
  (`/Engine/EditorBlueprintResources/StandardMacros.IsValid` _returnvalue
    (:`Is Valid`
      (`/Game/Blueprints/Farts/BP_FartBase.SetUp` _returnvalue _config self)
      (`/Game/Blueprints/Farts/BP_FartBase.Start` _returnvalue _config))))

(fn `FartDash`
  (params (Strength :type "Float (double-precision)") (Duration :type "Float (double-precision)") (`Airborne Speed Multiplier` :type "Float (double-precision)") (JumpHeightRatio :type "Float (double-precision)"))
  (if (not (`self.IsAirborne`))
    (`self.Jumped` `Airborne Speed Multiplier` (* Strength (`KismetMathLibrary.Normal2D` (`self.Directionality`))) (`local.Duration`) JumpHeightRatio)))

(fn `FartJump`
  (params (Strength :type "Float (double-precision)") (Duration :type "Float (double-precision)") (`Airborne Speed Multiplier` :type "Float (double-precision)") (JumpHeightRatio :type "Float (double-precision)"))
  (if (not (`self.IsAirborne`))
    (`self.Jumped` `Airborne Speed Multiplier` (* Strength (* (`KismetMathLibrary.Normal2D` (`KismetMathLibrary.Conv_VectorToVector2D` (`self.GetVelocity`))) (0.3 0.3))) Duration JumpHeightRatio)))

(fn `GetCanPickUpBeans`
  (returns (CanPickUp :type Boolean))
  (for _array_element (`/Game/Blueprints/Player/BP_ItemSlotState.Slots` (`self.ItemSlotState`))
    (if (`|EnumEquality` (`.FartType_22_E145F1A04CA5945F7C4608B8F584F25D` (break `/Game/Blueprints/Player/S_ItemSlotData` _array_element)) "NewEnumerator5")
      (return true)))
  (return false))

(fn `GetCanTakeDamageThisFrame`
  (returns (CanTakeDamage :type Boolean))
  (locals (IsOverlappingNonDisgustedEnemy :type Boolean))
  (bind _isoverlappingnondisgustedenemy (`self.GetIsOverlappingNonDisgustedEnemy`))
  (if _isoverlappingnondisgustedenemy
    (if (`self.IsAlive`)
      (bind _gamestate (`self.GetGameState`))
      (bind _isintrolevel (`/Game/Blueprints/GS_TopDown.GetIsIntroLevel` _gamestate))
      (if _isintrolevel
        _
        (else
          (return (and (not (`self.IsDamageBlinkActive`)) (not (`self.IsAirborne`))))))))
  (return false))

(fn `GetConfig`
  (params (Type :type "/Game/Blueprints/Farts/E_FartType Enum" :default "NewEnumerator5"))
  (returns (Config :type "/Game/Blueprints/Farts/S_FartConfig Structure"))
  (bind _gamestate (`self.GetGameState`))
  (bind _config (`/Game/Blueprints/GS_TopDown.GetFartConfig` _gamestate Type))
  (return _config))

(fn `GetGameState`
  (returns (GameState :type "/Game/Blueprints/GS_TopDown Object Reference"))
  (bind _asgs_top_down (cast `/Game/Blueprints/GS_TopDown` (`GameplayStatics.GetGameState`)))
  (return _asgs_top_down))

(fn `GetIsOverlappingEnemies`
  (returns (IsOverlapping :type Boolean))
  (return (not (`BlueprintSetLibrary.Set_IsEmpty` (`self.OverlappingEnemies`)))))

(fn `GetIsOverlappingNonDisgustedEnemy`
  (returns (IsOverlappingNonDisgustedEnemy :type Boolean))
  (bind _result (`BlueprintSetLibrary.Set_ToArray` (`self.OverlappingEnemies`)))
  (for _array_element _result
    (if (not (`/Game/Blueprints/Enemy/BP_EnemyBase.IsDisgusted` _array_element))
      (return true)))
  (return false))

(fn `GetSpeed`
  (returns (Speed :type "Float (double-precision)"))
  (return (* (`self.BaseSpeed`) (`self.SpeedMultiplier`))))

(fn `On Interact Pressed`
  (bind _lookedattrigger (`self.LookedAtTrigger`))
  (if (not (`self.IsAirborne`))
    (`/Engine/EditorBlueprintResources/StandardMacros.IsValid` _lookedattrigger
      (:`Is Valid`
        (`/Game/Blueprints/Interactions/BP_InteractionTriggerBase.Trigger` _lookedattrigger self)))))

(fn `OnAttackPressed`
  (params (Index :type Integer))
  (locals (LastTime :type "Float (double-precision)") (Config :type "/Game/Blueprints/Farts/S_FartConfig Structure") (Type :type "/Game/Blueprints/Farts/E_FartType Enum"))
  (bind _itemslotstate (`self.ItemSlotState`))
  (bind _data (`/Game/Blueprints/Player/BP_ItemSlotState.GetSlot` _itemslotstate Index))
  (if (`.CanBeTriggered_26_1548CDFA4D0215668F3C66AC88E5936A` (break `/Game/Blueprints/Player/S_ItemSlotData` _data))
    (`/Game/Blueprints/Player/BP_ItemSlotState.TriggerSlot` _itemslotstate (break `/Game/Blueprints/Player/S_ItemSlotData` _data))
    (`self.Fart` (`.FartType_22_E145F1A04CA5945F7C4608B8F584F25D` (break `/Game/Blueprints/Player/S_ItemSlotData` _data)))))

(fn `PickUpBeans`
  (params (IsSpecial :type Boolean))
  (locals (Type :type "/Game/Blueprints/Farts/E_FartType Enum"))
  (bind _slots (`/Game/Blueprints/Player/BP_ItemSlotState.Slots` (`self.ItemSlotState`)))
  (bind (_output_index _output_farttype) (break `/Game/Blueprints/Player/S_ItemSlotData` (`|GetArrayItem` _slots 2)))
  (bind (_output_index_2 _output_farttype_2) (break `/Game/Blueprints/Player/S_ItemSlotData` (`|GetArrayItem` _slots)))
  (bind (_output_index_3 _output_farttype_3) (break `/Game/Blueprints/Player/S_ItemSlotData` (`|GetArrayItem` _slots 1)))
  (if IsSpecial
    (set `local.Type` (`KismetArrayLibrary.Array_Random` (`|MakeArray` (enumliteral `/Game/Blueprints/Farts/E_FartType` "NewEnumerator1") (enumliteral `/Game/Blueprints/Farts/E_FartType` "NewEnumerator2") (enumliteral `/Game/Blueprints/Farts/E_FartType` "NewEnumerator3") (enumliteral `/Game/Blueprints/Farts/E_FartType` "NewEnumerator4"))))
    (else
      (set `local.Type` "NewEnumerator0")))
  (if (`|EnumEquality` _output_farttype_2 "NewEnumerator5")
    (`/Game/Blueprints/Player/BP_ItemSlotState.SetSlotItem` (`self.ItemSlotState`) (`local.Type`) 0)
    (elif (`|EnumEquality` _output_farttype_3 "NewEnumerator5")
      (`/Game/Blueprints/Player/BP_ItemSlotState.SetSlotItem` (`self.ItemSlotState`) (`local.Type`) 1)
      (elif (`|EnumEquality` _output_farttype "NewEnumerator5")
        (`/Game/Blueprints/Player/BP_ItemSlotState.SetSlotItem` (`self.ItemSlotState`) (`local.Type`) 2)
        (else
          (`KismetSystemLibrary.PrintString` "Trying to pickup can when there is no space!" true true (struct :`R` 0.846084 :`B` 1.0 :`A` 1.0)))))))

(fn `ReachedGoal`
  (if (not (`self.HasReachedGoal`))
    (set `self.HasReachedGoal` true)
    (bind _gamestate (`self.GetGameState`))
    (bind _isintrolevel (`/Game/Blueprints/GS_TopDown.GetIsIntroLevel` _gamestate))
    (if _isintrolevel
      (`/Game/Blueprints/GS_TopDown.ReachedIntroGoal` _gamestate)
      (`/Game/Blueprints/GS_TopDown.FadeOut` _gamestate)
      (else
        (`/Game/Blueprints/GS_TopDown.FadeOut` _gamestate)
        (`KismetSystemLibrary.K2_SetTimer` _gamestate "GoToNextLevel" 0.75)))))

(fn `StartDamageBlink`
  (set `self.IsDamageBlinkActive` true)
  (set `self.DamageBlinkEndTime` (+ (`GameplayStatics.GetTimeSeconds`) (- (`self.TakeDamageInterval`) 0.06)))
  (`self.UpdateDamageBlink`)
  (`KismetSystemLibrary.K2_SetTimer` null "EndDamageBlink" (`self.TakeDamageInterval`)))

(fn `ToggleAirborne`
  (params (IsAirborne :type Boolean) (AirborneSpeedMultiplier :type "Float (double-precision)") (JumpVelocity :type "Vector2D Structure"))
  (bind _output_get (set `self.IsAirborne` IsAirborne))
  (if _output_get
    (set `self.AirborneSpeedMultiplier` AirborneSpeedMultiplier)
    (set `self.JumpVelocity` JumpVelocity)
    (else
      (set `self.AirborneSpeedMultiplier` 1.0)
      (set `self.JumpVelocity` (0.0 0.0))))
  (`PrimitiveComponent.SetEnableGravity` (`self.CapsuleComponent`) (not (`self.IsAirborne`)))
  (`self.K2_SetActorLocation` (+ (`self.K2_GetActorLocation`) (`KismetMathLibrary.MakeVector` 0.0 0.0 4.0)) false true))

(fn `UpdateDamageBlink`
  (if (>= (`GameplayStatics.GetTimeSeconds`) (`self.DamageBlinkEndTime`))
    (`self.EndDamageBlink`)
    (else
      (if (`self.IsDamageBlinkRed`)
        (`PaperFlipbookComponent.SetSpriteColor` (`self.Sprite`) (`self.NormalColor`))
        (set `self.IsDamageBlinkRed` false)
        (else
          (`PaperFlipbookComponent.SetSpriteColor` (`self.Sprite`) (`self.DamageColor`))
          (set `self.IsDamageBlinkRed` true)))
      (`KismetSystemLibrary.K2_SetTimer` null "UpdateDamageBlink" (`self.DamageBlinkPeriod`)))))

(fn `UpdateJumpHeight`
  (locals (JumpProgress :type "Float (double-precision)") (TweenedProgress :type "Float (double-precision)"))
  (bind _returnvalue (- (`self.LandTime`) (`self.JumpTime`)))
  (bind (_relativelocation_x _relativelocation_y _relativelocation_z) (`KismetMathLibrary.BreakVector` (`SceneComponent.RelativeLocation` (`self.Sprite`))))
  (`SceneComponent.SetVisibility` (`self.Shadow`) (`self.IsAirborne`) false)
  (if (== _returnvalue 0.0)
    (set `local.JumpProgress` 0.0)
    (else
      (set `local.JumpProgress` (`KismetMathLibrary.FMin` (/ (- (`GameplayStatics.GetTimeSeconds`) (`self.JumpTime`)) _returnvalue) 1.0))))
  (set `local.TweenedProgress` (* (`KismetMathLibrary.Sin` (* (`local.JumpProgress`) (`KismetMathLibrary.GetPI`))) (`self.JumpHeightRatio`)))
  (`SceneComponent.K2_SetRelativeLocation` (`self.Sprite`) (`KismetMathLibrary.MakeVector` _relativelocation_x (- (`self.SpriteOffset`) (`KismetMathLibrary.Lerp` 0.0 (`self.MaxJumpPlayerOffset`) (`local.TweenedProgress`))) _relativelocation_z) false false)
  (`SceneComponent.SetRelativeScale3D` (`self.Shadow`) (* (`KismetMathLibrary.Vector_One`) (* (`self.ShadowScale`) (`KismetMathLibrary.Lerp` 1.0 (`self.MaxJumpShadowScale`) (`local.TweenedProgress`))))))

(fn `UpdateLookedAtTrigger`
  (locals (PreviousLookedAtTrigger :type "/Game/Blueprints/Interactions/BP_InteractionTriggerBase Object Reference"))
  (bind _previouslookedattrigger (`local.PreviousLookedAtTrigger`))
  (bind _lookedattrigger (`self.LookedAtTrigger`))
  (bind _returnvalue (`KismetSystemLibrary.IsValid` _lookedattrigger))
  (bind _output_get (set `local.PreviousLookedAtTrigger` (`self.LookedAtTrigger`)))
  (bind _trigger (`self.CalculateLookedAtTrigger`))
  (if (!= _trigger _output_get)
    (set `self.LookedAtTrigger` _trigger)
    (`self.On Interact Pressed`)
    (if (`KismetSystemLibrary.IsValid` _previouslookedattrigger)
      (`/Game/Blueprints/Interactions/BP_InteractionTriggerBase.SetIsLookedAt` _previouslookedattrigger false))
    (if _returnvalue
      (`/Game/Blueprints/Interactions/BP_InteractionTriggerBase.SetIsLookedAt` _lookedattrigger true))
    (bind _gamestate (`self.GetGameState`))
    (`/Game/Blueprints/UI/WBP_HUD.TogglePickUpPrompt` (`|ConvertAsset` (`/Game/Blueprints/GS_TopDown.HUD` _gamestate)) _returnvalue)))

(fn `UserConstructionScript`)